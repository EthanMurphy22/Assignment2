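; BP_GameItem is a game item actor, likely a block or cube, that can explode or respawn itself.
; DestroyEffect spawns an explosion effect at the actor's transform and destroys the actor.
; Spawn creates new BP_GameItem instances at the given location through both a DoOnce branch and a branch following self-destruction.
; Each spawn plays a cube sound at a hardcoded position, stores the new Block and calls CallBlockSpawned on it.
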(event `DestroyEffect`
  (`|SpawnActorFromClass` "/Game/StarterContent/Blueprints/Blueprint_Effect_Explosion.Blueprint_Effect_Explosion_C" (`self.GetTransform`) "AlwaysSpawn" "MultiplyWithRoot" null null)
  (`self.K2_DestroyActor`))

(event `Spawn`
  (params (SpawnLocation :type "Transform Structure"))
  (`|ExecutionSequence`
    (:`then_0`
      (`/Engine/EditorBlueprintResources/StandardMacros.DoOnce` false
        (:`Completed`
          _)))
    (:`then_1`
      (`self.K2_DestroyActor`)))
  (bind _returnvalue (`|SpawnActorFromClass` "BP_GameItem_C" SpawnLocation "AlwaysSpawn" "MultiplyWithRoot" null null))
  (`GameplayStatics.PlaySoundAtLocation` "/Game/SFX/SFX_CubeSpawn.SFX_CubeSpawn" (90.0 1455.0 935.0) (struct) 1.0 1.0 0.0 null null null null)
  (bind _output_get (set `self.Block` _returnvalue))
  (`self.BlockSpawned` _output_get))

(fn `DestroyEffect1`)

(fn `UserConstructionScript`)