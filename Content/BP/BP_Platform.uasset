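; Moving platform Blueprint that slides its static mesh along a local axis in one of three behaviors chosen by PlatformType.
; Type 1 makes a delayed, sounded X move and type 3 a short one, both reversible through PlatformBack.
; Type 2 travels along Y up to MaxDistance, replaying through an open gate.
; Animate uses a helper timeline to smoothly scrub that looping timeline to a given playback position.
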(event `Platform`
  (bind _staticmesh (`self.StaticMesh`))
  (bind _sfx_platform (`self.SFX_Platform`))
  (switch `/Game/PlatformEnum` (`self.PlatformType`)
    (:`NewEnumerator0`
      (`KismetSystemLibrary.Delay` 2.5)
      (`AudioComponent.Play` _sfx_platform 0.0)
      (bind (_direction _newtrack_0) (`Timeline|Timeline_1` :!label _label)
        (:`Update`
          (`SceneComponent.K2_SetRelativeLocation` _staticmesh (`KismetMathLibrary.MakeVector` (`KismetMathLibrary.Lerp` 0.0 1065.0 _newtrack_0)) false false))
        (:`Finished`
          (`AudioComponent.FadeOut` _sfx_platform 0.2 0.0 "Linear"))))
    (:`NewEnumerator1`
      (`AudioComponent.SetVolumeMultiplier` _sfx_platform 0.3)
      (`AudioComponent.Play` _sfx_platform 0.0)
      (bind (_direction_2 _newtrack_1) (`Timeline|Platform Timeline` :!label _label_2)
        (:`Update`
          (`SceneComponent.K2_SetRelativeLocation` _staticmesh (`KismetMathLibrary.MakeVector` 0.0 (`KismetMathLibrary.Lerp` 0.0 (`self.MaxDistance`) _newtrack_1)) false false))
        (:`Finished`
          (`/Engine/EditorBlueprintResources/StandardMacros.Gate` false
            (:`Exit`
              (goto _label_2 :!via `PlayFromStart`))))))
    (:`NewEnumerator3`
      (bind (_direction_3 _newtrack_0_2 _door) (`Timeline|Timeline` :!label _label_3)
        (:`Update`
          (`SceneComponent.K2_SetRelativeLocation` _staticmesh (`KismetMathLibrary.MakeVector` (`KismetMathLibrary.Lerp` 0.0 250.0 _door)) false false))))))

(event `PlatformBack`
  (switch `/Game/PlatformEnum` (`self.PlatformType`)
    (:`NewEnumerator0`
      (`AudioComponent.Play` (`self.SFX_Platform`) 0.0)
      (goto _label :!via `Reverse`))
    (:`NewEnumerator3`
      (goto _label_3 :!via `Reverse`))))

(event `Animate`
  (params (Location :type "Float (double-precision)"))
  (bind _platform_timeline (`self.Platform Timeline`))
  ;[1 1 1] Set Platform Delay
  (bind _output_get (set `self.CurrentPos` (`TimelineComponent.GetPlaybackPosition` _platform_timeline)))
  (bind (_direction _newtrack_0) (`Timeline|Timeline_0` :!via `PlayFromStart`)
    (:`Update`
      (`TimelineComponent.SetPlaybackPosition` _platform_timeline (`KismetMathLibrary.Lerp` _output_get Location _newtrack_0) false true))))

(fn `UserConstructionScript`)