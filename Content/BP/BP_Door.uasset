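; BP_Door is an interactable door that swings open and then moves the player on according to its DoorType.
; Interact plays a sound and starts a timeline that lerps the mesh yaw open.
; After a delay chained from the timeline's Update, a type switch either teleports the player back or opens another level, enabling cursor and UI input before the menu.
; An unconnected Room 3 level load never runs.
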(event `/Game/BP/BPI_Interface.Interact`
  (bind _returnvalue (`GameplayStatics.GetPlayerController` 0))
  (`GameplayStatics.PlaySoundAtLocation` "/Game/SFX/SFX_Door.SFX_Door" (0.0 0.0 0.0) (struct) 1.0 1.0 0.0 null null null null)
  (bind (_direction _doorfloat) (`Timeline|Timeline` :!via `PlayFromStart`)
    (:`Update`
      (`SceneComponent.K2_SetRelativeRotation` (`self.StaticMesh`) (`KismetMathLibrary.MakeRotator` 0.0 0.0 (`KismetMathLibrary.Lerp` 0.0 90.0 _doorfloat)) false false)
      (`KismetSystemLibrary.Delay` 0.6)
      (switch `/Game/DoorEnum` (`self.DoorType`)
        (:`NewEnumerator0`
          (`KismetSystemLibrary.Delay` 0.2)
          (bind _asbp_first_person_character (cast `/Game/FirstPerson/Blueprints/BP_FirstPersonCharacter` (`GameplayStatics.GetPlayerCharacter` 0)))
          (`self.K2_TeleportTo` _asbp_first_person_character (0.0 0.0 0.0) (struct :`Yaw` 90.0) :!pinned true) ; Teleport Player back to Player Start
        )
        (:`NewEnumerator1`
          (`GameplayStatics.OpenLevel` "Room2" :!pinned true) ; Advance to Room 2
        )
        (:`NewEnumerator2`
          (`WidgetBlueprintLibrary.SetInputMode_UIOnlyEx` _returnvalue null)
          (set `PlayerController.bShowMouseCursor` true _returnvalue)
          (`GameplayStatics.OpenLevel` "NewLevel" :!pinned true) ; Exit to Menu
        )
        (:`NewEnumerator4`
          (`GameplayStatics.OpenLevel` "Room1"))))))

(fn `UserConstructionScript`)